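; BP_ScorePickUp is a placeable pickup that adds its score value to the HUD when a third-person or grounded player overlaps it.
; On overlap it plays a pitch-randomized sound, spawns smoke, calls AddScoreToHUD on MyMainHUD and destroys itself.
; A Grounded flag makes the construction script use a randomly yawed dirt mesh; otherwise it uses the configured mesh, which a ping-ponging timeline bobs and spins.
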(event OnComponentBeginOverlap(StaticMesh)
  (params (OverlappedComponent :type Primitive%20Component%20Object%20Reference) (OtherActor :type Actor%20Object%20Reference) (OtherComp :type Primitive%20Component%20Object%20Reference) (OtherBodyIndex :type Integer) (bFromSweep :type Boolean) (SweepResult :type Hit%20Result%20Structure%20%28by%20ref%29))
  (Utilities|Casting|CastToBP_ThirdPersonPlayer OtherActor
    (:then
      _)
    (:CastFailed
      (Utilities|Casting|CastToBP_GroundedPlayer OtherActor)))
  (Audio|PlaySoundatLocation "/Game/KIT_Proto/MySound/PickUpSound/Cue/PickUp_Cue.PickUp_Cue" (Transformation|GetActorLocation) "0, 0, 0" 1.0 (Math|Random|RandomFloatinRange 1.0 1.25) 0.0 0 0 0 0)
  (Niagara|SpawnSystematLocation "/Game/KIT_Proto/Effects/PickUp/PickUpSmoke.PickUpSmoke" (Transformation|GetWorldLocation (Variables|Default|GetStaticMesh)))
  (bind _asmy_main_hud (Utilities|Casting|CastToMyMainHUD (HUD|GetHUD (Game|GetPlayerController 0))))
  (Default|AddScoretoHUD _asmy_main_hud (Variables|Construction|GetPickUpScoreValue))
  (Actor|DestroyActor))

(event EventBeginPlay
  (if (not (Variables|Construction|GetbGrounded))
    (bind _newtrack_0 (Timeline|upDownMovement PlayFromStart)
      (:Update
        (Transformation|SetRelativeLocation (Variables|Default|GetStaticMesh) (Math|Vector|MakeVector 0.0 0.0 (+ (Math|Float|Lerp 0.0 5e+01 _newtrack_0) 5e+01)) false false)
        (Class|Actor|AddActorWorldRotation "0.000000,0.500000,0.000000"))
      (:Finished
        (Utilities|FlowControl|FlipFlop
          (:A
            (Timeline|upDownMovement ReverseFromEnd))
          (:B
            (Timeline|upDownMovement PlayFromStart)))))))

(fn ConstructionScript
  (if (Variables|Construction|GetbGrounded)
    (Components|StaticMesh|SetStaticMesh (Variables|Default|GetStaticMesh) "/Game/KIT_Proto/MyMeshes/MSH_DirtGround.MSH_DirtGround")
    (Transformation|SetRelativeRotation (Variables|Default|GetStaticMesh) (Math|Rotator|MakeRotator 0.0 0.0 (Math|Random|RandomFloatinRange 0.0 1.8e+02)) false false)
    (else
      (Components|StaticMesh|SetStaticMesh (Variables|Default|GetStaticMesh) (Variables|Construction|GetMesh)))))