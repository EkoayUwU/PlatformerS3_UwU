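; Pawn for the player's burrowed state, which moves underground with camera-relative input, force feedback and a dirt mesh shown when movement stops.
; InitGroundedPlayer stores the original player and copies its camera orientation.
; Tick traces down against WorldDynamic to hold the capsule below the surface and the Niagara trail on it.
; Dig or Jump checks clearance above, then repossesses and launches the stored player and destroys this pawn, or shakes the camera if blocked.
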(event Custom|Init%20Grounded%20Player
  (params (PlayerRef :type BP%20Third%20Person%20Player%20Object%20Reference))
  (bind _capsulecomponent (Variables|Collision|GetCapsuleComponent))
  ;[0.151 0.151 0.151] Init Grounded Player
  (Variables|HiddenVariable|SetPlayerRef PlayerRef)
  (Transformation|SetWorldLocation _capsulecomponent (- (Transformation|GetWorldLocation _capsulecomponent) "0.000000,0.000000,200.000000") false false)
  (Transformation|SetRelativeRotation _capsulecomponent (Math|Rotator|MakeRotator (.roll (Class|SpringArmComponent|GetTargetRotation (Variables|/Game/KIT_Proto/Core/Character/BP_ThirdPersonPlayer.BP_ThirdPersonPlayer_C|GetCameraBoom (Variables|HiddenVariable|GetPlayerRef)))) 0.0 (.yaw (Class|SpringArmComponent|GetTargetRotation (Variables|/Game/KIT_Proto/Core/Character/BP_ThirdPersonPlayer.BP_ThirdPersonPlayer_C|GetCameraBoom (Variables|HiddenVariable|GetPlayerRef))))) false false)
  (Transformation|SetWorldTransform (Variables|Default|GetCameraBoom) (Math|Transform|MakeTransform (+ (.location (Transformation|GetWorldTransform (Variables|/Game/KIT_Proto/Core/Character/BP_ThirdPersonPlayer.BP_ThirdPersonPlayer_C|GetCameraBoom (Variables|HiddenVariable|GetPlayerRef)))) "0.000000,0.000000,65.000000") (.rotation (Transformation|GetWorldTransform (Variables|/Game/KIT_Proto/Core/Character/BP_ThirdPersonPlayer.BP_ThirdPersonPlayer_C|GetCameraBoom (Variables|HiddenVariable|GetPlayerRef)))) (.scale (Transformation|GetWorldTransform (Variables|/Game/KIT_Proto/Core/Character/BP_ThirdPersonPlayer.BP_ThirdPersonPlayer_C|GetCameraBoom (Variables|HiddenVariable|GetPlayerRef))))) false false))

(event Input|EnhancedActionEvents|EnhancedInputActionIA_Move
  (params (ActionValue :type Vector%202D%20Structure) (ElapsedSeconds :type Float%20%28double-precision%29) (TriggeredSeconds :type Float%20%28double-precision%29) (InputAction :type Input%20Action%20Object%20Reference :default "/Game/KIT_Proto/Core/Character/Inputs/IA_Move.IA_Move"))
  (bind _returnvalue (Pawn|GetControlRotation :!class /Script/Engine.Pawn))
  ;[0.151 0.151 0.151] Input Movement
  (:Triggered
    (Pawn|Input|AddMovementInput (Math|Vector|RotateVector (Math|Vector|MakeVector (.x ActionValue) 0.0 0.0) (Math|Rotator|MakeRotator 0.0 0.0 (.yaw _returnvalue))) 1.0 false)
    (Pawn|Input|AddMovementInput (Math|Vector|RotateVector (Math|Vector|MakeVector 0.0 (.y ActionValue) 0.0) (Math|Rotator|MakeRotator 0.0 0.0 (.yaw _returnvalue))) 1.0 false)
    (if (or (not (Math|Float|InRange(Float) (.x (Transformation|GetVelocity)) -3e+01 3e+01)) (not (Math|Float|InRange(Float) (.y (Transformation|GetVelocity)) -3e+01 3e+01)))
      ;[0 0.2838 1] Controller Shake
      (Game|Feedback|ClientPlayForceFeedback (Game|GetPlayerController 0) "/Game/KIT_Proto/Core/Character/ControllerShake/InGroundFB.InGroundFB" "None" false false false)
      (Rendering|SetVisibility (Variables|Default|GetMSH_DirtGround) false false)))
  (:Canceled
    (Rendering|SetVisibility (Variables|Default|GetMSH_DirtGround) true false :!label _label))
  (:Completed
    (goto _label)))

(event Input|EnhancedActionEvents|EnhancedInputActionIA_Dig
  (params (ActionValue :type Boolean) (ElapsedSeconds :type Float%20%28double-precision%29) (TriggeredSeconds :type Float%20%28double-precision%29) (InputAction :type Input%20Action%20Object%20Reference :default "/Game/KIT_Proto/Core/Character/Inputs/IA_Dig.IA_Dig"))
  (bind _cameraboom (Variables|Default|GetCameraBoom))
  (bind _playerref (Variables|HiddenVariable|GetPlayerRef))
  (bind _playerref_2 (Variables|HiddenVariable|GetPlayerRef))
  (bind _returnvalue (Class|SpringArmComponent|GetTargetRotation _cameraboom))
  (bind _capsulecomponent (Variables|/Script/Engine.Character|GetCapsuleComponent _playerref_2))
  ;[0.151 0.151 0.151] Get Out Of Ground
  (:Started
    (bind _bcangetoutofground (CallFunction|CheckifCanGetOutOfGround))
    (if _bcangetoutofground
      ;;[0.5469 0.5469 0.5469] Re Enable Player
      (Default|EnablePlayer (Variables|HiddenVariable|GetPlayerRef))
      (Transformation|SetWorldLocation _capsulecomponent (+ (Variables|Default|GetOut%20Hit%20Impact%20Point) "0.000000,0.000000,100.000000") false false)
      (Transformation|SetRelativeRotation _capsulecomponent (Math|Rotator|MakeRotator (.roll _returnvalue) 0.0 (.yaw _returnvalue)) false false)
      (Pawn|Possess (Game|GetPlayerController 0) (Variables|HiddenVariable|GetPlayerRef))
      (Character|LaunchCharacter _playerref (+ (Variables|/Script/Engine.MovementComponent|GetVelocity (Variables|Character|GetCharacterMovement)) "0.000000,0.000000,420.000000") false false)
      (Variables|/Game/KIT_Proto/Core/Character/BP_ThirdPersonPlayer.BP_ThirdPersonPlayer_C|SetJumpCount _playerref 1)
      (Actor|DestroyActor)
      (else
        ;;[0.9323 0 0] Add Cam Shake + Noise
        (Camera|PlayWorldCameraShake "/Game/KIT_Proto/Core/Character/BP_CameraShake.BP_CameraShake_C" (Transformation|GetWorldLocation (Variables|Default|GetCamera)) 0.0 5e+02)))))

(event Input|EnhancedActionEvents|EnhancedInputActionIA_Look
  (params (ActionValue :type Vector%202D%20Structure) (ElapsedSeconds :type Float%20%28double-precision%29) (TriggeredSeconds :type Float%20%28double-precision%29) (InputAction :type Input%20Action%20Object%20Reference :default "/Game/KIT_Proto/Core/Character/Inputs/IA_Look.IA_Look"))
  ;[0.151 0.151 0.151] Input Look
  (Pawn|Input|AddControllerYawInput (.x ActionValue))
  (Pawn|Input|AddControllerPitchInput (.y ActionValue)))

(event Input|EnhancedActionEvents|EnhancedInputActionIA_Jump
  (params (ActionValue :type Boolean) (ElapsedSeconds :type Float%20%28double-precision%29) (TriggeredSeconds :type Float%20%28double-precision%29) (InputAction :type Input%20Action%20Object%20Reference :default "/Game/KIT_Proto/Core/Character/Inputs/IA_Jump.IA_Jump"))
  (bind _cameraboom (Variables|Default|GetCameraBoom))
  (bind _playerref (Variables|HiddenVariable|GetPlayerRef))
  (bind _playerref_2 (Variables|HiddenVariable|GetPlayerRef))
  (bind _returnvalue (Class|SpringArmComponent|GetTargetRotation _cameraboom))
  (bind _capsulecomponent (Variables|/Script/Engine.Character|GetCapsuleComponent _playerref_2))
  ;[0.151 0.151 0.151] Get Out Of Ground
  (:Started
    (bind _bcangetoutofground (CallFunction|CheckifCanGetOutOfGround))
    (if _bcangetoutofground
      ;;[0.5469 0.5469 0.5469] Re Enable Player
      (Default|EnablePlayer (Variables|HiddenVariable|GetPlayerRef))
      (Transformation|SetWorldLocation _capsulecomponent (+ (Variables|Default|GetOut%20Hit%20Impact%20Point) "0.000000,0.000000,100.000000") false false)
      (Transformation|SetRelativeRotation _capsulecomponent (Math|Rotator|MakeRotator (.roll _returnvalue) 0.0 (.yaw _returnvalue)) false false)
      (Pawn|Possess (Game|GetPlayerController 0) (Variables|HiddenVariable|GetPlayerRef))
      (Character|LaunchCharacter _playerref (+ (Variables|/Script/Engine.MovementComponent|GetVelocity (Variables|Character|GetCharacterMovement)) "0.000000,0.000000,420.000000") false false)
      (Variables|/Game/KIT_Proto/Core/Character/BP_ThirdPersonPlayer.BP_ThirdPersonPlayer_C|SetJumpCount _playerref 1)
      (Actor|DestroyActor)
      (else
        ;;[0.9323 0 0] Add Cam Shake + Noise
        (Camera|PlayWorldCameraShake "/Game/KIT_Proto/Core/Character/BP_CameraShake.BP_CameraShake_C" (Transformation|GetWorldLocation (Variables|Default|GetCamera)) 0.0 5e+02)))))

(event EventTick
  (params (DeltaSeconds :type Float%20%28single-precision%29))
  (bind _raycastguizmo (Variables|Default|GetRaycastGuizmo))
  (bind _returnvalue (Transformation|GetWorldLocation _raycastguizmo))
  ;[0.151 0.151 0.151] Set Player Height Level
  (Utilities|FlowControl|Sequence
    (:then_0
      (bind (_outhit _returnvalue_2) (Collision|LineTraceForObjects _returnvalue (- _returnvalue "0.000000,0.000000,500.000000") (Utilities|Array|MakeArray "ObjectTypeQuery2") false 0 "None"))
      (bind _output_get (Variables|Default|SetOut%20Hit%20Impact%20Point (.impactpoint _outhit)))
      (Transformation|SetWorldLocation (Variables|Collision|GetCapsuleComponent) (- _output_get "0.000000,0.000000,175.000000") false false)
      (if _returnvalue_2
        (Transformation|SetWorldLocation (Variables|Default|GetNS_GroundTrail) (.impactpoint _outhit) false false)))))

(fn ConstructionScript)

(fn CheckifCanGetOutOfGround
  (bind _out_hit_impact_point (Variables|Default|GetOut%20Hit%20Impact%20Point))
  (bind _returnvalue (Collision|LineTraceForObjects (+ _out_hit_impact_point "0.000000,0.000000,10.000000") (+ _out_hit_impact_point "0.000000,0.000000,200.000000") (Utilities|Array|MakeArray "ObjectTypeQuery1" "ObjectTypeQuery2") false 0 "None"))
  (return (not _returnvalue)))