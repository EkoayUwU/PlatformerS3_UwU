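; BP_PickUp is a pickup prop that spins and bobs until a player collects it.
; Tick applies a steady world rotation, while a self-retriggering FlipFlop alternately plays a timeline forward and in reverse to lerp the mesh height.
; Mesh overlap by BP_ThirdPersonPlayer or BP_GroundedPlayer plays a randomly pitched sound, spawns smoke and destroys the actor, with no reward logic here.
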(event OnComponentBeginOverlap(StaticMesh)
  (params (OverlappedComponent :type Primitive%20Component%20Object%20Reference) (OtherActor :type Actor%20Object%20Reference) (OtherComp :type Primitive%20Component%20Object%20Reference) (OtherBodyIndex :type Integer) (bFromSweep :type Boolean) (SweepResult :type Hit%20Result%20Structure%20%28by%20ref%29))
  (Utilities|Casting|CastToBP_ThirdPersonPlayer OtherActor
    (:then
      _)
    (:CastFailed
      (Utilities|Casting|CastToBP_GroundedPlayer OtherActor)))
  (Audio|PlaySoundatLocation "/Game/MyContents/MySound/PickUpSound/Cue/PickUp_Cue.PickUp_Cue" (Transformation|GetActorLocation) "0, 0, 0" 1.0 (Math|Random|RandomFloatinRange 1.0 1.25) 0.0 0 0 0 0)
  (Niagara|SpawnSystematLocation "/Game/MyContents/MyNiagara/PickUp/PickUpSmoke.PickUpSmoke" (Transformation|GetWorldLocation (Variables|Default|GetStaticMesh)))
  (Actor|DestroyActor))

(event Custom|UpDownAnim
  (Utilities|FlowControl|FlipFlop
    (:A
      (bind _newtrack_0 (Timeline|Timeline PlayFromStart)
        (:Update
          (Transformation|SetRelativeLocation (Variables|Default|GetStaticMesh) (Math|Vector|MakeVector 0.0 0.0 (+ (Math|Float|Lerp 0.0 5e+01 _newtrack_0) 5e+01)) false false))
        (:Finished
          (CallFunction|UpDownAnim))))
    (:B
      (Timeline|Timeline ReverseFromEnd))))

(event EventBeginPlay
  (CallFunction|UpDownAnim))

(event EventTick
  (params (DeltaSeconds :type Float%20%28single-precision%29))
  (Class|Actor|AddActorWorldRotation "0.000000,0.500000,0.000000"))

(fn ConstructionScript)