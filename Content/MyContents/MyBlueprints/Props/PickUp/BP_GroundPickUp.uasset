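; Ground pickup prop that awards score when a third-person or grounded player overlaps its box.
; On pickup it plays a pitch-randomized sound, spawns smoke at the dirt ground mesh, adds its score value through the main HUD, then destroys itself.
; A DoOnce gate runs before the player casts, so the first overlap by any actor uses up the trigger.
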(event OnComponentBeginOverlap(Box)
  (params (OverlappedComponent :type Primitive%20Component%20Object%20Reference) (OtherActor :type Actor%20Object%20Reference) (OtherComp :type Primitive%20Component%20Object%20Reference) (OtherBodyIndex :type Integer) (bFromSweep :type Boolean) (SweepResult :type Hit%20Result%20Structure%20%28by%20ref%29))
  (Utilities|FlowControl|DoOnce false
    (:Completed
      (Utilities|Casting|CastToBP_ThirdPersonPlayer OtherActor
        (:then
          _)
        (:CastFailed
          (Utilities|Casting|CastToBP_GroundedPlayer OtherActor)))
      (Audio|PlaySoundatLocation "/Game/MyContents/MySound/PickUpSound/Cue/PickUp_Cue.PickUp_Cue" (Transformation|GetActorLocation) "0, 0, 0" 1.0 (Math|Random|RandomFloatinRange 1.0 1.25) 0.0 0 0 0 0)
      (Niagara|SpawnSystematLocation "/Game/MyContents/MyNiagara/PickUp/PickUpSmoke.PickUpSmoke" (Transformation|GetWorldLocation (Variables|Default|GetMSH_DirtGround)))
      (bind _asmy_main_hud (Utilities|Casting|CastToMyMainHUD (HUD|GetHUD (Game|GetPlayerController 0))))
      (Default|AddScoretoHUD _asmy_main_hud (Variables|Default|GetPickUpScoreValue))
      (Actor|DestroyActor))))

(event EventBeginPlay)

(event Collision|EventActorBeginOverlap
  (params (OtherActor :type Actor%20Object%20Reference)))

(event EventTick
  (params (DeltaSeconds :type Float%20%28single-precision%29)))

(fn ConstructionScript)