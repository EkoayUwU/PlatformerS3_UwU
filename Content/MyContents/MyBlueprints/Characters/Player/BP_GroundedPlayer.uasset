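; BP_GroundedPlayer is a player character Blueprint that handles basic movement and look input through Enhanced Input.
; On BeginPlay it adds the IMC_Player mapping context to the first player controller's local player subsystem.
; IA_Move adds movement along the control rotation's yaw-only forward and right axes, ignoring camera pitch.
; IA_Look feeds its X and Y values into controller yaw and pitch.
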(event Input|EnhancedActionEvents|EnhancedInputActionIA_Move
  (params (ActionValue :type Vector%202D%20Structure) (ElapsedSeconds :type Float%20%28double-precision%29) (TriggeredSeconds :type Float%20%28double-precision%29) (InputAction :type Input%20Action%20Object%20Reference :default "/Game/MyContents/MyBlueprints/Characters/Player/Inputs/IA_Move.IA_Move"))
  (bind _returnvalue (Pawn|GetControlRotation :!class /Script/Engine.Pawn))
  ;[0.151 0.151 0.151] Input Movement
  (Pawn|Input|AddMovementInput (Math|Vector|RotateVector (Math|Vector|MakeVector (.x ActionValue) 0.0 0.0) (Math|Rotator|MakeRotator 0.0 0.0 (.yaw _returnvalue))) 1.0 false)
  (Pawn|Input|AddMovementInput (Math|Vector|RotateVector (Math|Vector|MakeVector 0.0 (.y ActionValue) 0.0) (Math|Rotator|MakeRotator 0.0 0.0 (.yaw _returnvalue))) 1.0 false))

(event Input|EnhancedActionEvents|EnhancedInputActionIA_Look
  (params (ActionValue :type Vector%202D%20Structure) (ElapsedSeconds :type Float%20%28double-precision%29) (TriggeredSeconds :type Float%20%28double-precision%29) (InputAction :type Input%20Action%20Object%20Reference :default "/Game/MyContents/MyBlueprints/Characters/Player/Inputs/IA_Look.IA_Look"))
  ;[0.151 0.151 0.151] Input Look
  (Pawn|Input|AddControllerYawInput (.x ActionValue))
  (Pawn|Input|AddControllerPitchInput (.y ActionValue)))

(event EventBeginPlay
  ;[0.151 0.151 0.151] Init IMC
  (Input|AddMappingContext (PlayerController|LocalPlayerSubsystems|GetEnhancedInputLocalPlayerSubsystem (Game|GetPlayerController 0)) "/Game/MyContents/MyBlueprints/Characters/Player/IMC_Player.IMC_Player" 0 "(bIgnoreAllPressedKeysUntilRelease=True,bForceImmediately=False,bNotifyUserSettings=False)"))

(fn ConstructionScript)